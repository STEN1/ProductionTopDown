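; Ghoul enemy Blueprint that manages the character's health bar widget.
; On BeginPlay it casts the Widget1 component's user widget to WBP_CharHealthBar, stores it, constructs it with itself as owner and applies HealthBarScale as render scale.
; A RemoveHealthBar event hides the stored widget when the reference is valid.
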(event EventBeginPlay
  (bind _aswbp_char_health_bar (Utilities|Casting|CastToWBP_CharHealthBar (UserInterface|GetUserWidgetObject (Variables|Default|GetWidget1))))
  (Variables|Default|SetHealthBarRef _aswbp_char_health_bar)
  (Default|ConstructHealthbar (Variables|Default|GetHealthBarRef) self)
  (Widget|Transform|SetRenderScale (Variables|Default|GetHealthBarRef) (Variables|Default|GetHealthBarScale)))

(event EventRemoveHealthBar
  (bind _healthbarref (Variables|Default|GetHealthBarRef))
  (Utilities|IsValid _healthbarref
    (:Is%20Valid
      (Widget|SetVisibility _healthbarref "Hidden"))))

(fn ConstructionScript)