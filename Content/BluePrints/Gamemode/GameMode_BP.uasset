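; GameMode Blueprint that owns the player HUD and end-of-game screen.
; StartGame creates and caches the health bar and inventory widgets and adds them to the viewport.
; Custom events forward health, stamina, inventory slot selection and slot image updates to those cached widgets.
; GameOver spawns a game-over widget and sets its text from whether the player won.
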(event EventUpdateHealthUI
  (params (Health :type Float%20%28single-precision%29) (DefaultHealth :type Float%20%28single-precision%29))
  (Default|UpdateHealthbar (Variables|Default|GetHealthBarRef) Health DefaultHealth))

(event EventUpdateStaminaUI
  (params (Stamina :type Float%20%28single-precision%29) (DefaultStamina :type Float%20%28single-precision%29))
  (Default|UpdateStaminabar (Variables|Default|GetHealthBarRef) Stamina DefaultStamina))

(event EventStartGame
  (bind _returnvalue (UserInterface|CreateWidget "/Game/BluePrints/Widgets/Healthbar/WBP_Healthbar.WBP_Healthbar_C"))
  (Variables|Default|SetHealthBarRef _returnvalue)
  (UserInterface|Viewport|AddtoViewport _returnvalue 0)
  (bind _returnvalue_2 (UserInterface|CreateWidget "/Game/BluePrints/Widgets/Inventory/WBP_Inventory.WBP_Inventory_C"))
  (Variables|Default|SetInventoryRef _returnvalue_2)
  (UserInterface|Viewport|AddtoViewport _returnvalue_2 0))

(event EventGameOver
  (params (PlayerWon :type Boolean))
  (bind _returnvalue (UserInterface|CreateWidget "/Game/BluePrints/Widgets/GameOver/WBP_GameOver.WBP_GameOver_C"))
  (Default|SetGameOverText _returnvalue PlayerWon)
  (UserInterface|Viewport|AddtoViewport _returnvalue 0))

(event EventUpdateInventoryUI
  (params (Slot :type Integer) (ItemImage :type Texture%202D%20Object%20Reference))
  (Default|SetImageSlot (Variables|Default|GetInventoryRef) Slot ItemImage))

(event EventUpdateInventoryUICurrentSlot
  (params (CurrentSlot :type Integer))
  (Default|SetCurrentSlot (Variables|Default|GetInventoryRef) CurrentSlot))

(fn ConstructionScript)