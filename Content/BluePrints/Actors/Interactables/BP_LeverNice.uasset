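; BP_LeverNice is a lever interactable that shows a "Use" prompt when the player is near.
; On BeginPlay it sets the text of its WBP_ItemWidget and hides the widget component.
; Actor overlap events toggle the widget's visibility as a PlayerCharacter enters or leaves.
; The graph contains only this prompt logic, with no lever activation behavior.
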(event EventBeginPlay
  (bind _aswbp_item_widget (Utilities|Casting|CastToWBP_ItemWidget (UserInterface|GetUserWidgetObject (Variables|Default|GetWidget))))
  (Default|SetItemText _aswbp_item_widget "Use")
  (Rendering|SetVisibility (Variables|Default|GetWidget) false false))

(event Collision|EventActorBeginOverlap
  (params (OtherActor :type Actor%20Object%20Reference))
  (Utilities|Casting|CastToPlayerCharacter OtherActor)
  (Rendering|SetVisibility (Variables|Default|GetWidget) true false))

(event Collision|EventActorEndOverlap
  (params (OtherActor :type Actor%20Object%20Reference))
  (Utilities|Casting|CastToPlayerCharacter OtherActor)
  (Rendering|SetVisibility (Variables|Default|GetWidget) false false))

(fn ConstructionScript)