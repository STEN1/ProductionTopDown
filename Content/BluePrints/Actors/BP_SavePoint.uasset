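; BP_SavePoint is a save point actor that briefly shows an on-screen save indicator when its OnSaved event fires.
; It creates the WBP_SaveGameIcon widget on first use, caches it and hides it after a short delay.
; Later calls reuse the cached widget, toggling its visibility only when it is not already showing.
; The graph contains only this feedback, with no save or trigger logic.
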(event EventOnSaved
  (if (Utilities|IsValid (Variables|Default|GetSaveGameIcon))
    (if (not (Widget|IsVisible (Variables|Default|GetSaveGameIcon)))
      (Widget|SetVisibility (Variables|Default|GetSaveGameIcon) "Visible")
      (Utilities|FlowControl|Delay 2.0)
      (Widget|SetVisibility (Variables|Default|GetSaveGameIcon) "Hidden"))
    (else
      (bind _returnvalue (UserInterface|CreateWidget "/Game/BluePrints/Widgets/SavingIcon/WBP_SaveGameIcon.WBP_SaveGameIcon_C"))
      (bind _output_get (Variables|Default|SetSaveGameIcon _returnvalue))
      (UserInterface|Viewport|AddtoViewport _output_get 0)
      (Utilities|FlowControl|Delay 2.0)
      (Widget|SetVisibility (Variables|Default|GetSaveGameIcon) "Hidden"))))

(fn ConstructionScript)